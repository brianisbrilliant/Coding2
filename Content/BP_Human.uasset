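; BP_Human is a human actor with a rudimentary attack, taking input from the first player controller.
; Pressing Attack or activating the root component prints a debug string, then loops over all BP_Human actors.
; It calls TakeDamage on those differing from the activation event's Component, rather than from self.
; The following health-style check compares two zero literals, so DestroyActor always follows the damage call, with no explicit target.
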(event `InputAction|Attack`
  (params (Key :type "Key Structure"))
  (:`Pressed`
    (`KismetSystemLibrary.PrintString` "Starting Blueprint" :!label _label)
    (bind _outactors (`GameplayStatics.GetAllActorsOfClass` "BP_Human_C"))
    (for _array_element _outactors
      (if (!= _array_element (stale `self.DefaultSceneRoot.OnComponentActivated` Component))
        (`self.TakeDamage` _array_element)
        (if (not (> 0.0 0.0))
          (`self.K2_DestroyActor`))))))

(event `self.ReceiveBeginPlay`
  (`self.EnableInput` (`GameplayStatics.GetPlayerController` 0)))

(event `self.DefaultSceneRoot.OnComponentActivated`
  (params (Component :type "ActorComponent Object Reference") (bReset :type Boolean))
  (goto _label))

(fn `UserConstructionScript`)