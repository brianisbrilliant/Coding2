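; Save manager that writes and restores BP_BlueCube transforms through a BP_SaveGame slot.
; Save input copies its CubeTransforms array into a new save object, but an existing slot leaves TheSaveGame None, so the cast stops the save.
; BeginPlay and load input read the slot unconditionally, then nested loops apply every transform to every cube, leaving all at the last one.
; Nothing here gathers cube transforms; a per-cube Save loop is unconnected.
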(event `InputAction|SaveGame`
  (params (Key :type "Key Structure"))
  (:`Pressed`
    (`self.Save Game`)))

(event `InputAction|LoadGame`
  (params (Key :type "Key Structure"))
  (:`Released`
    (`self.Load Game` :!label _label)))

(event `self.ReceiveBeginPlay`
  (goto _label))

(event `Save Game`
  (bind _returnvalue (`GameplayStatics.DoesSaveGameExist` (`self.SlotName`)))
  (if _returnvalue
    (`GameplayStatics.LoadGameFromSlot` (`self.SlotName`))
    (set `self.TheSaveGame` null)
    (else
      (bind _returnvalue_2 (`GameplayStatics.CreateSaveGameObject` "/Game/BP_SaveGame.BP_SaveGame_C"))
      (set `self.TheSaveGame` _returnvalue_2)))
  (bind _asbp_save_game (cast `/Game/BP_SaveGame` (`self.TheSaveGame`)))
  (set `/Game/BP_SaveGame.CubeTransforms` (`self.CubeTransforms`) _asbp_save_game)
  (`GameplayStatics.SaveGameToSlot` (`self.TheSaveGame`) (`self.SlotName`)))

(event `Load Game`
  (`GameplayStatics.DoesSaveGameExist` (`self.SlotName`))
  (if true
    (bind _returnvalue (`GameplayStatics.LoadGameFromSlot` (`self.SlotName`)))
    (bind _asbp_save_game (cast `/Game/BP_SaveGame` _returnvalue))
    (bind _output_get (set `self.CubeTransforms` (`/Game/BP_SaveGame.CubeTransforms` _asbp_save_game))) ; Then, find all cubes and set their transforms.
    (`|ExecutionSequence`
      (:`then_0`
        (bind _outactors (`GameplayStatics.GetAllActorsOfClass` "/Game/BP_BlueCube.BP_BlueCube_C")))
      (:`then_1`
        (for _array_element _output_get
          (for _array_element_2 _outactors :!label _label_2
            (`self.K2_SetActorTransform` _array_element_2 _array_element false false)))
        (goto _label_2 :!via `Break`)))))

(fn `UserConstructionScript`)